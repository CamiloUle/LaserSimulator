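; Laser engraver lab actor that engraves a BP_TableToSpawn placed inside it.
; A timeline toggles the cover; while open, a Box overlap snaps the table into place and disables its physics.
; With the cover closed, timelines move carrier and laser with sound and Niagara sparks, then change the table's material.
; Tick colors cover and panel outlines by state and, on a Delay, restores table physics once engraving finishes and the cover opens.
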(event `self.ReceiveBeginPlay`
  (bind _table (`self.Table`))
  (set `self.InitialLocation` (`SceneComponent.K2_GetComponentLocation` (`self.Carrier`)))
  (set `self.InitialLaserLocation` (`SceneComponent.K2_GetComponentLocation` (`self.Laser`)))
  (set `self.InitialCoverRotation` (`SceneComponent.K2_GetComponentRotation` (`self.Cover`)))
  (`SceneComponent.SetVisibility` (`self.Cylinder`) false false)
  (`SceneComponent.SetVisibility` _table false false)
  (set `self.LocationToTable` (`SceneComponent.K2_GetComponentLocation` _table))
  (set `self.RotationToTable` (`SceneComponent.K2_GetComponentRotation` _table)))

(event `self.ReceiveTick`
  (params (DeltaSeconds :type "Float (single-precision)"))
  (bind _coverchild (`self.CoverChild`))
  (bind _controlpanel (`self.ControlPanel`))
  (`|ExecutionSequence`
    (:`then_0`
      (if (`self.bCanOpenCover`)
        (`MeshComponent.SetOverlayMaterial` _coverchild "/Game/Media/Materials/M_GreenOutline.M_GreenOutline")
        (else
          (`MeshComponent.SetOverlayMaterial` _coverchild "/Game/Media/Materials/M_RedOutline.M_RedOutline"))))
    (:`then_1`
      (if (`self.bIsTraceWithPanel`)
        (`MeshComponent.SetOverlayMaterial` _controlpanel "/Game/Media/Materials/M_GreenOutline.M_GreenOutline")
        (else
          (`MeshComponent.SetOverlayMaterial` _controlpanel "/Game/Media/Materials/M_RedOutline.M_RedOutline"))))
    (:`then_2`
      (`KismetSystemLibrary.Delay` 3.0)
      (`self.EnablePhysicsOnTable`))))

(event `self.OnPlayTimelineCover`
  (bind (_initialcoverrotation_roll _initialcoverrotation_pitch _initialcoverrotation_yaw) (`KismetMathLibrary.BreakRotator` (`self.InitialCoverRotation`)))
  ;[1 0.05429 0] OpenCover
  (if (`self.bCanOpenCover`)
    (set `self.bCoverWasOpen` true)
    (`/Engine/EditorBlueprintResources/StandardMacros.FlipFlop`
      (:`A`
        (bind (_direction _newtrack_0) (`Timeline|CoverTimeline` :!via `PlayFromStart` :!label _label)
          (:`Update`
            (`SceneComponent.K2_SetWorldRotation` (`self.Cover`) (`KismetMathLibrary.MakeRotator` _initialcoverrotation_roll (`KismetMathLibrary.Lerp` 0.0 _newtrack_0 -50.0) _initialcoverrotation_yaw) false false))))
      (:`B`
        (set `self.bCoverWasOpen` false)
        (goto _label :!via `Reverse`)))))

(event `self.Box.OnComponentBeginOverlap`
  (params (OverlappedComponent :type "PrimitiveComponent Object Reference") (OtherActor :type "Actor Object Reference") (OtherComp :type "PrimitiveComponent Object Reference") (OtherBodyIndex :type Integer) (bFromSweep :type Boolean) (SweepResult :type "HitResult Structure (by ref)"))
  ;[0.03899 0 1] OverlapToCheckTable
  (if (`self.bCoverWasOpen`)
    (bind _asbp_table_to_spawn (cast `/Game/Actors/BP_TableToSpawn` OtherActor))
    (`/Engine/EditorBlueprintResources/StandardMacros.IsValid` _asbp_table_to_spawn
      (:`Is Valid`
        (set `self.TableActor` _asbp_table_to_spawn)
        (bind _table (`/Game/Actors/BP_TableToSpawn.Table` _asbp_table_to_spawn))
        (set `self.TableActorComponent` _table)
        (`SceneComponent.K2_SetWorldLocationAndRotation` _table (`self.LocationToTable`) (struct :`Pitch` 90.0 :`Roll` -90.0) false false)
        (`PrimitiveComponent.SetSimulatePhysics` _table false)
        (set `self.bTableWasPutOnLaser` true)))))

(event `self.OnPlayTimelineLaser`
  (bind _tableactor (`self.TableActor`))
  ;[1 0.0603 0.9063] AnimLaser
  (set `self.bEngravingHasFinish` false)
  (if (`self.bCoverWasOpen`)
    _
    (elif (`self.bTableWasPutOnLaser`)
      (`KismetSystemLibrary.Delay` 1.5)
      (`self.PlaySound`)
      (`|ExecutionSequence`
        (:`then_0`
          (bind (_direction _newtrack_0) (`Timeline|CarrierTimeline` :!via `PlayFromStart` :!label _label_2)
            (:`Update`
              (bind _returnvalue (* _newtrack_0 -10.0))
              (bind _output_get (set `self.LocationToMove` (+ (`self.InitialLocation`) (`KismetMathLibrary.MakeVector` 0.0 _returnvalue))))
              (`SceneComponent.K2_SetWorldLocation` (`self.Carrier`) _output_get false false))
            (:`Finished`
              (`SceneComponent.K2_SetWorldLocation` (`self.Carrier`) (`self.InitialLocation`) false false)
              (set `self.bEngravingHasFinish` true))))
        (:`then_1`
          (bind (_direction_2 _alphamovementlaser) (`Timeline|LaserTimeline` :!via `PlayFromStart` :!label _label_3)
            (:`Update`
              (bind _output_get_2 (set `self.LocationToMoveLaser` (+ (`self.InitialLaserLocation`) (`KismetMathLibrary.MakeVector` (* _alphamovementlaser 10.0) _returnvalue))))
              (`SceneComponent.K2_SetWorldLocation` (`self.Laser`) _output_get_2 false false)
              (`SceneComponent.SetVisibility` (`self.Cylinder`) true false)
              (`NiagaraFunctionLibrary.SpawnSystemAtLocation` (`self.SparksNiagara`) (`SceneComponent.K2_GetComponentLocation` (`self.PoitNiagara`))))
            (:`Finished`
              (`SceneComponent.K2_SetWorldLocation` (`self.Laser`) (`self.InitialLaserLocation`) false false)
              (`SceneComponent.SetVisibility` (`self.Cylinder`) false false)
              (`AudioComponent.StopDelayed` (`self.AudioComponent`) 1.0)
              (`/Engine/EditorBlueprintResources/StandardMacros.IsValid` _tableactor
                (:`Is Valid`
                  (`/Game/Actors/BP_TableToSpawn.SetTableMaterial` _tableactor))))))))))

(event `self.Box.OnComponentEndOverlap`
  (params (OverlappedComponent :type "PrimitiveComponent Object Reference") (OtherActor :type "Actor Object Reference") (OtherComp :type "PrimitiveComponent Object Reference") (OtherBodyIndex :type Integer))
  ;[0.03899 0 1] OverlapToCheckTable
  (bind _asbp_table_to_spawn (cast `/Game/Actors/BP_TableToSpawn` OtherActor))
  (`/Engine/EditorBlueprintResources/StandardMacros.IsValid` _asbp_table_to_spawn
    (:`Is Valid`
      (set `self.bTableWasPutOnLaser` false))))

(event `self.OnStopTimeLineLaser`
  (bind _audiocomponent (`self.AudioComponent`))
  ;[1 0.0603 0.9063] AnimLaser
  (`/Engine/EditorBlueprintResources/StandardMacros.IsValid` _audiocomponent
    (:`Is Valid`
      (`AudioComponent.Stop` _audiocomponent)
      (`|ExecutionSequence`
        (:`then_0`
          (goto _label_2 :!via `Stop`))
        (:`then_1`
          (goto _label_3 :!via `Stop`))))))

(fn `CloseCover`
  (if (`self.bEngravingHasFinish`)
    _))

(fn `EnablePhysicsOnTable`
  (bind _tableactorcomponent (`self.TableActorComponent`))
  (`/Engine/EditorBlueprintResources/StandardMacros.IsValid` _tableactorcomponent
    (:`Is Valid`
      (if (and (`self.bEngravingHasFinish`) (`self.bCoverWasOpen`))
        (`PrimitiveComponent.SetSimulatePhysics` _tableactorcomponent true)
        (set `self.bEngravingHasFinish` false)))))

(fn `PlaySound`
  (bind _returnvalue (`GameplayStatics.CreateSound2D` (`self.Sound`) 1.0 1.0 0.0 null))
  (bind _output_get (set `self.AudioComponent` _returnvalue))
  (`AudioComponent.Play` _output_get 0.0))

(fn `UserConstructionScript`)