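; BP_Laser is an actor that animates a laser mounted on a moving carrier, starting four seconds after BeginPlay.
; Two timelines play together: one slides the carrier along world Y, the other offsets the laser along world X.
; The laser update also reads the carrier timeline's alpha, so the laser follows the carrier's Y motion.
; Each part returns to its cached starting location when its timeline finishes.
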(event `self.ReceiveBeginPlay`
  (set `self.InitialLocation` (`SceneComponent.K2_GetComponentLocation` (`self.LaserCarrier`)))
  (set `self.InitialLaserLocation` (`SceneComponent.K2_GetComponentLocation` (`self.Laser`)))
  (`KismetSystemLibrary.Delay` 4.0)
  (`|ExecutionSequence`
    (:`then_0`
      (bind (_direction _alphamovement) (`Timeline|CarrierTimeline`)
        (:`Update`
          (bind _returnvalue (* _alphamovement -15.0))
          (bind _output_get (set `self.LocationToMove` (+ (`self.InitialLocation`) (`KismetMathLibrary.MakeVector` 0.0 _returnvalue))))
          (`SceneComponent.K2_SetWorldLocation` (`self.LaserCarrier`) _output_get false false))
        (:`Finished`
          (`SceneComponent.K2_SetWorldLocation` (`self.LaserCarrier`) (`self.InitialLocation`) false false))))
    (:`then_1`
      (bind (_direction_2 _alphamovementlaser) (`Timeline|LaserTimeline`)
        (:`Update`
          (bind _output_get_2 (set `self.LocationToMoveLaser` (+ (`self.InitialLaserLocation`) (`KismetMathLibrary.MakeVector` (* _alphamovementlaser -10.0) _returnvalue))))
          (`SceneComponent.K2_SetWorldLocation` (`self.Laser`) _output_get_2 false false))
        (:`Finished`
          (`SceneComponent.K2_SetWorldLocation` (`self.Laser`) (`self.InitialLaserLocation`) false false))))))

(fn `UserConstructionScript`)