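; Table actor that shows a player-loaded texture through an engraving or cutting material.
; Tick sets the table's overlay to a green or red outline according to CanChangeMaterial.
; SetMaterial reads CanStartEngraving on BP_PlayerController to pick the engrave or cut base for a dynamic material instance.
; If the controller's LoadedTexture is valid, it feeds that into the instance and applies it to the table.
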(event `self.ReceiveTick`
  (params (DeltaSeconds :type "Float (single-precision)"))
  (bind _table (`self.Table`))
  (if (`self.bCanChangeMaterial`)
    (`MeshComponent.SetOverlayMaterial` _table "/Game/Media/Materials/M_GreenOutline.M_GreenOutline")
    (else
      (`MeshComponent.SetOverlayMaterial` _table "/Game/Media/Materials/M_RedOutline.M_RedOutline"))))

(event `self.ReceiveBeginPlay`)

(fn `SetMaterial`
  (bind _table (`self.Table`))
  (bind _table_2 (`self.Table`))
  (bind _asbp_player_controller (cast `/Game/General/BP_PlayerController` (`GameplayStatics.GetPlayerController` 0)))
  (`/Engine/EditorBlueprintResources/StandardMacros.IsValid` _asbp_player_controller
    (:`Is Valid`
      (if (`LSPlayerController.bCanStartEngraving` _asbp_player_controller)
        (bind _returnvalue (`PrimitiveComponent.CreateDynamicMaterialInstance` _table 0 "/Game/Media/Materials/M_GravMaterial.M_GravMaterial" "None"))
        (set `self.Material` _returnvalue)
        (bind _loadedtexture (`LSPlayerController.LoadedTexture` _asbp_player_controller))
        (`/Engine/EditorBlueprintResources/StandardMacros.IsValid` _loadedtexture
          (:`Is Valid`
            (`MaterialInstanceDynamic.SetTextureParameterValue` _returnvalue "TextureParam" _loadedtexture)
            (`PrimitiveComponent.SetMaterial` _table 0 (`self.Material`))))
        (else
          (bind _returnvalue_2 (`PrimitiveComponent.CreateDynamicMaterialInstance` _table_2 0 "/Game/Media/Materials/M_CutMaterial.M_CutMaterial" "None"))
          (set `self.Material` _returnvalue_2)
          (`/Engine/EditorBlueprintResources/StandardMacros.IsValid` _loadedtexture
            (:`Is Valid`
              (`MaterialInstanceDynamic.SetTextureParameterValue` _returnvalue_2 "TextureParam" _loadedtexture)
              (`PrimitiveComponent.SetMaterial` _table_2 0 (`self.Material`)))))))))

(fn `UserConstructionScript`)