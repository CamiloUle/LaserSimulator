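; Door actor that swings open when OnOpenDoor fires and reverses after a ten-second delay.
; A timeline lerps world yaw from zero to the Offeset variable, keeping the pitch and roll cached at BeginPlay but not the initial yaw.
; Timeline Finished triggers the delayed ReverseFromEnd and also fires after reversing, so the closing swing repeats from the open position.
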(event `self.ReceiveBeginPlay`
  (set `self.InitialRotation` (`SceneComponent.K2_GetComponentRotation` (`self.Door`))))

(event `self.OnOpenDoor`
  (bind (_initialrotation_roll _initialrotation_pitch) (`KismetMathLibrary.BreakRotator` (`self.InitialRotation`)))
  (bind (_direction _doormovement) (`Timeline|Timeline` :!label _label)
    (:`Update`
      (`SceneComponent.K2_SetWorldRotation` (`self.Door`) (`KismetMathLibrary.MakeRotator` _initialrotation_roll _initialrotation_pitch (`KismetMathLibrary.Lerp` 0.0 (`self.Offeset`) _doormovement)) false false))
    (:`Finished`
      (`KismetSystemLibrary.Delay` 10.0)
      (goto _label :!via `ReverseFromEnd`))))

(fn `UserConstructionScript`)